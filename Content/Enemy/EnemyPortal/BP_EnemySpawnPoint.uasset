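; BP_EnemySpawnPoint is a portal spawn point that telegraphs and then spawns one BP_Enemy_Base each time its routine is triggered.
; StartSpawnRoutine calls the SpawnRoutine event, which plays beam VFX and sound and swaps SPortal2 materials to light up the portal.
; After a configurable delay it restores the cached inactive material, then spawns the enemy with a zap effect at a Z offset.
; IsSpawning stays true throughout the routine.
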(event `self.ReceiveBeginPlay`
  (set `self.inactive_Material` (`PrimitiveComponent.GetMaterial` (`self.S_Portal2`) 1)))

(event `SpawnRoutine`
  (bind _returnvalue (`SceneComponent.K2_GetComponentLocation` (`self.S_Portal2`)))
  (set `self.IsSpawning` true)
  (`self.SpawnPortalVisuals` _returnvalue)
  (`GameplayStatics.PlaySoundAtLocation` "/Game/Audio/Sounds/Objects/MS_Portal.MS_Portal" _returnvalue (struct) 1.0 1.0 0.0 null null null null)
  (`PrimitiveComponent.SetMaterial` (`self.S_Portal2`) 1 "/Game/Enemy/EnemyPortal/M_Portal_Light_Circle.M_Portal_Light_Circle")
  (`KismetSystemLibrary.Delay` (`self.PortalSpawnDelayAfterVisual`))
  (`PrimitiveComponent.SetMaterial` (`self.S_Portal2`) 1 (`self.inactive_Material`))
  (bind _location (`self.GetSpawnLocation`))
  (`self.SpawnEnemy` (`KismetMathLibrary.MakeTransform` _location))
  (set `self.IsSpawning` false))

(fn `GetSpawnLocation`
  (returns (Location :type "Vector Structure"))
  (return (+ (`SceneComponent.K2_GetComponentLocation` (`self.S_Portal2`)) (`KismetMathLibrary.MakeVector` 0.0 0.0 (`self.zOffset`)))))

(fn `SpawnEnemy`
  (params (SpawnTransform :type "Transform Structure"))
  (bind _location (`self.GetSpawnLocation`))
  (`NiagaraFunctionLibrary.SpawnSystemAtLocation` "/Game/VFX/Vefects/Zap_VFX/VFX/Zap/Particles/NS_Zap_01_Red.NS_Zap_01_Red" _location)
  (`|SpawnActorFromClass` "/Game/Enemy/BP_Enemy_Base.BP_Enemy_Base_C" SpawnTransform "Undefined" "MultiplyWithRoot" null null)
  (`PrimitiveComponent.SetMaterial` (`self.S_Portal2`) 2 "/Engine/EditorLandscapeResources/AlphaBrushMaterial_Smooth.AlphaBrushMaterial_Smooth"))

(fn `SpawnPortalVisuals`
  (params (Location :type "Vector Structure"))
  (`|ExecutionSequence`
    (:`then_0`
      (bind _location (`self.GetSpawnLocation`))
      (`NiagaraFunctionLibrary.SpawnSystemAtLocation` "/Game/VFX/NS_Portalbeam.NS_Portalbeam" _location))
    (:`then_1`
      (`PrimitiveComponent.SetMaterial` (`self.S_Portal2`) 2 "/Game/Props/Materials/PinkProvet.PinkProvet"))))

(fn `StartSpawnRoutine`
  (`self.SpawnRoutine`))

(fn `UserConstructionScript`
  (`parent.UserConstructionScript`))