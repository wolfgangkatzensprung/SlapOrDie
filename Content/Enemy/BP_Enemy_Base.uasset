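; Base multiplayer slap enemy that chases a random player, slaps in melee with sphere traces and hitstop, and retries when stuck.
; Incoming slaps replicate a timed physics ragdoll with impulse; the capsule follows the body via ground traces.
; Standing up uses a pose snapshot and front/back orientation, then resumes the chase.
; Death notifies game mode, credits the last slapper, and multicasts score popup and death-reason effects.
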(event `self.ReceiveBeginPlay`
  ; Init
  (`self.InitPhysicsSetup`)
  (`self.ChasePlayer`)
  (`self.InitStuckCheckLoop`))

(event `InitPhysicsSetup`
  ; Init
  (set `self.RootBoneOffset` (`SceneComponent.RelativeLocation` (`self.Mesh`)))
  (`SkeletalMeshComponent.SetAllBodiesSimulatePhysics` (`self.Mesh`) false))

(event `ChasePlayer`
  ; Chase
  (set `self.IsStuck` false)
  (bind _asgm_slap_game_mode (cast `/Game/Slappedy/GM_SlapGameMode` (`GameplayStatics.GetGameMode`)))
  (bind _rndplayer (`/Game/Slappedy/GM_SlapGameMode.GetRandomPlayer` _asgm_slap_game_mode))
  (`|AIMoveTo` self (0.0 0.0 0.0) _rndplayer 150.0
    (:`OnSuccess`
      (`self.Server_Attack`)
      (`KismetSystemLibrary.Delay` 2.0)
      (`self.ChasePlayer`))
    (:`OnFail`
      (if (`KismetMathLibrary.BooleanNAND` (`self.isRagdolling`) (`self.IsSlapping`))
        (set `self.IsStuck` true)))))

(event `InitStuckCheckLoop`
  ; Init
  (if (`self.IsStuck`) :!label _label
    (`self.ChasePlayer`))
  (`KismetSystemLibrary.Delay` (`self.StuckCheckDelay`))
  (goto _label))

(event `Server_Attack`
  ; Server Attack
  (`self.MC_Attack`))

(event `self.ReceiveTick`
  (params (DeltaSeconds :type "Float (single-precision)"))
  ; Tick
  (`self.UpdateCapsuleLoc`))

(event `MC_Attack`
  ; Client Multicast Attack
  (`|ExecutionSequence`
    (:`then_0`
      ; Attack Animation
      (bind _asabp_slap_enemy (cast `/Game/Enemy/Slap_Enemy/ABP_Slap_Enemy` (`SkeletalMeshComponent.GetAnimInstance` (`self.Mesh`))))
      (`/Game/Enemy/Slap_Enemy/ABP_Slap_Enemy.StartSlap` _asabp_slap_enemy)
      (`KismetSystemLibrary.Delay` (`self.SlapAnimationTime`))
      (`/Game/Enemy/Slap_Enemy/ABP_Slap_Enemy.StopSlap` _asabp_slap_enemy))
    (:`then_1`
      ; Attack Logic
      (`KismetSystemLibrary.Delay` 0.4)
      (`self.TryPerformSlap`))))

(event `Server_OnSlapped`
  (params (SlapForce :type "Vector Structure") (Actor :type "Actor Object Reference"))
  ; Slapped -> Ragdoll
  (`self.MC_SlappedFeedback` SlapForce)
  (bind _asbp_slap_player (cast `/Game/Player/Prof/BP_Slap_Player` Actor)
    (:`then`
      (set `self.LastPlayerWhoSlapped` _asbp_slap_player))
    (:`CastFailed`
      (set `self.LastPlayerWhoSlapped` null)))
  (set `self.isRagdolling` true)
  (`KismetSystemLibrary.DelayUntilNextTick`)
  (`self.MC_ApplySlapImpulse` SlapForce)
  (`KismetSystemLibrary.RetriggerableDelay` 3.0)
  (set `self.isRagdolling` false))

(event `StandupRoutine`
  ; Stand Up after Ragdolling
  (`self.StartStandUp`)
  (`KismetSystemLibrary.DelayUntilNextTick`)
  (`self.ResetToStanding`))

(event `MC_SlappedFeedback`
  (params (SlapForce :type "Vector Structure"))
  ; Slapped -> Ragdoll
  (`self.PlayHurtSound`)
  (bind _returnvalue (`NiagaraFunctionLibrary.SpawnSystemAtLocation` "/Game/VFX/NS_getslapped.NS_getslapped" (+ (`SceneComponent.K2_GetComponentLocation` (`self.Mesh`)) (0.0 0.0 200.0))))
  (`NiagaraComponent.SetVariableVec3` _returnvalue "Direction" SlapForce))

(event `PlayHurtSound`
  ; SFX
  (`GameplayStatics.PlaySoundAtLocation` "/Game/Audio/Sounds/Hurt/MS_EnemyHurt.MS_EnemyHurt" (0.0 0.0 0.0) (struct) 1.0 1.0 0.0 null null null null))

(event `MC_ApplySlapImpulse`
  (params (Impulse :type "Vector Structure"))
  ; Slapped Force
  (`KismetSystemLibrary.DelayUntilNextTick`)
  (`PrimitiveComponent.AddImpulse` (`self.Mesh`) Impulse (`self.PhysicsBoneName`) false))

(event `Server_OnDeath`
  (params (DeathInfo :type "/Game/Slappedy/Struct_DeathInfo Structure"))
  (bind (_trapid _deathreason _lastslappingplayer) (break `/Game/Slappedy/Struct_DeathInfo` DeathInfo))
  ; Death
  (if (not (`self.IsDead`))
    (set `self.IsDead` true)
    (`self.MC_OnDeath` DeathInfo)
    (`self.NotifyGameMode_Death`)
    (`self.NotifyPlayerState_Death` _trapid _lastslappingplayer)
    (`self.GrantScore`)))

(event `/Game/Slappedy/BPI_BaseCharacter.StandUpFinished_Anim`
  ; Reset and get back to chase after stand up
  (if (not (`self.isRagdolling`))
    (`KismetSystemLibrary.Delay` 0.5)
    (`self.OnStandUpFinished`)))

(event `MC_OnDeath`
  (params (DeathInfo :type "/Game/Slappedy/Struct_DeathInfo Structure"))
  (bind (_trapid _deathreason) (break `/Game/Slappedy/Struct_DeathInfo` DeathInfo))
  (bind _mesh (`self.Mesh`))
  (bind _returnvalue (`SceneComponent.K2_GetComponentLocation` _mesh))
  (bind _returnvalue_2 (`SceneComponent.K2_GetComponentLocation` (`self.Mesh`)))
  (bind _asbp_player_state (cast `/Game/Player/BP_PlayerState` (`Pawn.PlayerState` (`self.LastPlayerWhoSlapped`)) :!pure true))
  (bind (_playerdata_playername _playerdata_playercontroller _playerdata_playernumber _playerdata_color) (break `/Game/Slappedy/Struct_PlayerData` (`/Game/Player/BP_PlayerState.PlayerData` _asbp_player_state)))
  ; Death
  (`|ExecutionSequence`
    (:`then_0`
      (`KismetSystemLibrary.Delay` 3.0)
      (`self.K2_DestroyActor`))
    (:`then_1`
      ; Death Number
      (`TextRenderComponent.SetTextRenderColor` (`self.Text_Plus1`) (`BlueprintMapLibrary.Map_Find` (`self.PlayerColorMaterial`) _playerdata_color))
      (`TextRenderComponent.K2_SetText` (`self.Text_Plus1`) (`|FormatText` "+{Score}" (* (`/Game/Player/BP_PlayerState.Multiplier` _asbp_player_state) (`self.ScorePoints`))))
      (`GameplayStatics.PlaySoundAtLocation` "/Game/Audio/Sounds/Feedback/Score01.Score01" _returnvalue_2 (struct) 1.0 1.0 0.0 null null null null)
      (`SceneComponent.K2_SetWorldLocationAndRotation` (`self.Text_Plus1`) _returnvalue_2 (struct :`Pitch` 30.0 :`Yaw` -130.0) false false)
      (`SceneComponent.SetVisibility` (`self.Text_Plus1`) true false)
      (bind (_direction _position _worldsize) (`Timeline|PlusScoreAnimationTimeline` :!via `PlayFromStart`)
        (:`Update`
          (`SceneComponent.K2_AddWorldTransform` (`self.Text_Plus1`) (`KismetMathLibrary.MakeTransform` (`KismetMathLibrary.MakeVector` 0.0 0.0 _position)) false false)
          (`TextRenderComponent.SetWorldSize` (`self.Text_Plus1`) (`|EaseFunction` "EaseInOut" _worldsize 0.0 36.0)))))
    (:`then_2`
      ;[0.0683 0.15 0.06405 0.5] Spawn Death Particles
      (switch `/Game/Slappedy/Enum_DeathReason` _deathreason
        (:`NewEnumerator0`
          (bind _returnvalue_3 (`NiagaraFunctionLibrary.SpawnSystemAttached` "/Game/VFX/NS_zapperdeath.NS_zapperdeath" _mesh "None" (0.0 0.0 0.0) (struct) "KeepRelativeOffset"))
          (`NiagaraFunctionLibrary.OverrideSystemUserVariableSkeletalMeshComponent` _returnvalue_3 "SKM" _mesh)
          (`SceneComponent.SetVisibility` (`self.Mesh`) false false))
        (:`NewEnumerator2`
          (`NiagaraFunctionLibrary.SpawnSystemAtLocation` "/Game/VFX/NS_firepitdeath.NS_firepitdeath" _returnvalue)
          (`SceneComponent.SetVisibility` (`self.Mesh`) false false))
        (:`NewEnumerator3`
          (`KismetSystemLibrary.PrintString` (`|GetEnumeratorNameAsString` _deathreason))
          (`NiagaraFunctionLibrary.SpawnSystemAtLocation` "/Game/VFX/NS_cauldrondeath.NS_cauldrondeath" _returnvalue))
        (:`NewEnumerator1`
          (`KismetSystemLibrary.Delay` 1.0)
          (`NiagaraFunctionLibrary.SpawnSystemAtLocation` "/Game/VFX/NS_Grinderdeathwall.NS_Grinderdeathwall" _returnvalue))
        (:`NewEnumerator5`
          (`KismetSystemLibrary.Delay` 2.0)
          (`NiagaraFunctionLibrary.SpawnSystemAtLocation` "/Game/VFX/NS_Grinderdeath.NS_Grinderdeath" _returnvalue))))))

(event `self.Mesh.OnComponentBeginOverlap`
  (params (OverlappedComponent :type "PrimitiveComponent Object Reference") (OtherActor :type "Actor Object Reference") (OtherComp :type "PrimitiveComponent Object Reference") (OtherBodyIndex :type Integer) (bFromSweep :type Boolean) (SweepResult :type "HitResult Structure (by ref)"))
  ; Enemy try find Deathzone when ragdolling bc he is invisible to Deathzone in this state.
)

(fn `CalculateSlapForce`
  (params (PlayerLocation :type "Vector Structure"))
  (returns (SlapForce :type "Vector Structure"))
  (return (+ (* (`KismetMathLibrary.Normal` (- PlayerLocation (`self.K2_GetActorLocation`))) (* (`self.SlapForce`) 100000.0)) (`self.SlapForceConstAdd`))))

(fn `EndHitstop`
  (set `self.CustomTimeDilation` 1.0))

(fn `FindCharacterOrientation`
  (bind (_returnvalue_x _returnvalue_y _returnvalue_z) (`KismetMathLibrary.BreakVector` (`KismetMathLibrary.GetRightVector` (`SceneComponent.GetSocketRotation` (`self.Mesh`) "pelvis"))))
  (set `self.IsLayingOnBack` (> _returnvalue_z 0.0)))

(fn `GetCanBeSlapped`
  (returns (CanBeSlapped :type Boolean))
  (return true))

(fn `GetCharacterMovementComponent`
  (returns (CharacterMovement :type "CharacterMovementComponent Object Reference"))
  (return (`self.CharacterMovement`)))

(fn `GetDoIK`
  (returns (DoIK :type Boolean))
  (return (`self.DoIK`)))

(fn `GetIsBeingSlapped`
  (returns (IsBeingSlapped :type Boolean))
  (return (`self.isRagdolling`)))

(fn `GetIsLayingOnBack`
  (returns (IsLayingOnBack :type Boolean))
  (return (`self.IsLayingOnBack`)))

(fn `GetIsRagdolling`
  (returns (IsRagdolling :type Boolean))
  (return (`self.isRagdolling`)))

(fn `GrantScore`
  (bind _lastplayerwhoslapped (`self.LastPlayerWhoSlapped`))
  (if (`KismetSystemLibrary.IsValid` _lastplayerwhoslapped)
    (bind _asbp_player_state (cast `/Game/Player/BP_PlayerState` (`Pawn.PlayerState` _lastplayerwhoslapped)))
    (`/Game/Player/BP_PlayerState.AddScore` _asbp_player_state (`self.ScorePoints`))))

(fn `NotifyGameMode_Death`
  (bind _asgm_slap_game_mode (cast `/Game/Slappedy/GM_SlapGameMode` (`GameplayStatics.GetGameMode`)))
  (`/Game/Slappedy/GM_SlapGameMode.OnEnemyDeath` _asgm_slap_game_mode))

(fn `NotifyPlayerState_Death`
  (params (TrapId :type String) (Player :type "Character Object Reference"))
  (`/Engine/EditorBlueprintResources/StandardMacros.IsValid` Player
    (:`Is Valid`
      (bind _asbp_player_state (cast `/Game/Player/BP_PlayerState` (`Pawn.PlayerState` Player)))
      (`/Game/Player/BP_PlayerState.OnEnemyKill` _asbp_player_state TrapId))))

(fn `OnRep_IsDead`
  (`self.StartRagdolling`))

(fn `OnRep_isRagdolling`
  (if (`self.isRagdolling`)
    (`self.StartRagdolling`)
    (else
      (`self.StandupRoutine`))))

(fn `OnStandUpFinished`
  (`CharacterMovementComponent.SetMovementMode` (`self.CharacterMovement`) "MOVE_Walking" 0)
  (`self.ChasePlayer`))

(fn `ResetToStanding`
  (`SkeletalMeshComponent.SetAllBodiesSimulatePhysics` (`self.Mesh`) false)
  (`PrimitiveComponent.SetCollisionEnabled` (`self.Mesh`) "NoCollision")
  (`PrimitiveComponent.SetCollisionEnabled` (`self.CapsuleComponent`) "QueryAndPhysics"))

(fn `SetCapsuleOrientation`
  (bind _mesh (`self.Mesh`))
  (bind _returnvalue (- (`SceneComponent.GetSocketLocation` _mesh "head") (`SceneComponent.GetSocketLocation` _mesh (`self.PhysicsBoneName`))))
  (`SceneComponent.K2_SetWorldRotation` (`self.CapsuleComponent`) (`KismetMathLibrary.MakeRotFromZX` (`KismetMathLibrary.MakeVector` 0.0 0.0 1.0) (`KismetMathLibrary.SelectVector` (* _returnvalue -1.0) _returnvalue (`self.IsLayingOnBack`))) false false))

(fn `StartHitstop`
  (set `self.CustomTimeDilation` 0.1)
  (`KismetSystemLibrary.K2_SetTimer` null "EndHitstop" (`self.HitstopTime`)))

(fn `StartRagdolling`
  (`PrimitiveComponent.SetCollisionEnabled` (`self.Mesh`) "QueryAndPhysics")
  (`SkeletalMeshComponent.SetAllBodiesBelowSimulatePhysics` (`self.Mesh`) (`self.RootBoneName`) true true)
  (`CharacterMovementComponent.DisableMovement` (`self.CharacterMovement`)))

(fn `StartStandUp`
  (if (and (`self.isRagdolling`) (not (`self.IsDead`)))
    (`self.FindCharacterOrientation`)
    (`self.SetCapsuleOrientation`)
    (`AnimInstance.SavePoseSnapshot` (`SkeletalMeshComponent.GetAnimInstance` (`self.Mesh`)) "RagdollFinalPose")))

(fn `TryApplySlap`
  (params (SlapForce :type "Vector Structure") (Slapper :type "Actor Object Reference"))
  (returns (SlapSucceeded :type Boolean))
  (`|ExecutionSequence`
    (:`then_0`
      (`self.Server_OnSlapped` SlapForce Slapper))
    (:`then_2`
      (return true))))

(fn `TryKill`
  (params (Killer :type "Actor Object Reference") (TrapId :type String) (DeathReason :type "/Game/Slappedy/Enum_DeathReason Enum" :default "NewEnumerator4"))
  (returns (Killed :type Boolean))
  (if (not (`self.IsDead`))
    (`self.Server_OnDeath` (make `/Game/Slappedy/Struct_DeathInfo` TrapId DeathReason (`self.LastPlayerWhoSlapped`)))
    (return true)
    (else
      (return false))))

(fn `TryPerformSlap`
  (returns (SlapSucceeded :type Boolean))
  (locals (SlappedSomething :type Boolean))
  (bind _returnvalue (`self.K2_GetActorLocation`))
  (if (not (`self.isRagdolling`))
    ; Find Targets
    (bind (_outhits _returnvalue_2) (`KismetSystemLibrary.SphereTraceMultiForObjects` :`Start` _returnvalue :`End` (+ _returnvalue (* (`KismetMathLibrary.GetForwardVector` (`self.K2_GetActorRotation`)) (`self.SlapRange`))) :`Radius` (`self.SlapRadius`) :`ObjectTypes` (`|MakeArray` "ObjectTypeQuery3" "ObjectTypeQuery6" :!type "EObjectTypeQuery Enum") :`DrawTime` 1.5))
    (if _returnvalue_2
      (`self.StartHitstop`)
      ; Slap each Player
      (for _array_element _outhits
        (bind (_bblockinghit _binitialoverlap _time _distance _location _impactpoint _normal _impactnormal _physmat _hitactor _hitcomponent) (`GameplayStatics.BreakHitResult` _array_element))
        (if (or (`self.ActorHasTag` _hitactor (`self.PlayerTag`)) (`KismetSystemLibrary.DoesImplementInterface` _hitactor "/Game/Slappedy/BPI_Breakable.BPI_Breakable_C"))
          (if (`KismetSystemLibrary.DoesImplementInterface` (`ActorComponent.GetOwner` _hitcomponent) "/Game/Slappedy/BPI_Slappable.BPI_Slappable_C")
            (bind _slapforce (`self.CalculateSlapForce` (`self.K2_GetActorLocation` _hitactor)))
            (bind _slapsucceeded (message `/Game/Slappedy/BPI_Slappable.TryApplySlap` _hitactor _slapforce self))
            (if _slapsucceeded
              (set `local.SlappedSomething` true)))))
      (return (`local.SlappedSomething`))
      (else
        (return false)))))

(fn `UpdateCapsuleLoc`
  (bind _returnvalue (`SceneComponent.GetSocketLocation` (`self.Mesh`) (`self.PhysicsBoneName`)))
  (if (`self.isRagdolling`)
    (bind (_outhit _returnvalue_2) (`KismetSystemLibrary.LineTraceSingle` :`Start` _returnvalue :`End` (+ _returnvalue (0.0 0.0 -100.0)) :`TraceChannel` "TraceTypeQuery1" :`DrawTime` 0.1))
    (if _returnvalue_2
      (set `self.TargetGroundLocation` (`.Location` (`GameplayStatics.BreakHitResult` _outhit)))
      (else
        (set `self.TargetGroundLocation` (`SceneComponent.GetSocketLocation` (`self.Mesh`) (`self.PhysicsBoneName`)))))
    (bind _output_get (set `self.MeshLocation` (- (`self.TargetGroundLocation`) (`self.RootBoneOffset`))))
    (`SceneComponent.K2_SetWorldLocation` (`self.CapsuleComponent`) _output_get false false)))

(fn `UserConstructionScript`)