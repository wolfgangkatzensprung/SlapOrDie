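; Electric barrier Blueprint that flashes beam effects between two sphere components, Sphere and SphereB.
; Tick calls UpdateTraces, which acts whenever the trace cooldown has elapsed.
; Each pass spawns an auto-destroying NS_electricbarrier Niagara system, setting its beam endpoints at random heights above each sphere, within MinRadius.
; A visibility line trace also runs between the spheres, but its result does not affect the beams.
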(event `self.ReceiveTick`
  (params (DeltaSeconds :type "Float (single-precision)"))
  (`self.UpdateTraces`))

(fn `UpdateTraces`
  (locals (RandomDirection :type "Vector Structure" :default (0.0 0.0 0.0)) (ImpactOffset :type "Float (double-precision)" :default 1.0))
  (bind _returnvalue (`KismetMathLibrary.MakeVector` (.x (`SceneComponent.K2_GetComponentLocation` (`self.Sphere`))) (.y (`SceneComponent.K2_GetComponentLocation` (`self.Sphere`))) (+ (.z (`SceneComponent.K2_GetComponentLocation` (`self.Sphere`))) (* (`KismetMathLibrary.RandomFloat`) (`self.MinRadius`)))))
  (bind _returnvalue_2 (`KismetMathLibrary.MakeVector` (.x (`SceneComponent.K2_GetComponentLocation` (`self.SphereB`))) (.y (`SceneComponent.K2_GetComponentLocation` (`self.SphereB`))) (+ (.z (`SceneComponent.K2_GetComponentLocation` (`self.SphereB`))) (* (`KismetMathLibrary.RandomFloat`) (`self.MinRadius`)))))
  ; check cooldown
  (if (>= (- (`GameplayStatics.GetTimeSeconds`) (`self.LastTrace`)) (`self.TraceCooldown`))
    (`KismetSystemLibrary.LineTraceSingle` :`Start` _returnvalue :`End` _returnvalue_2 :`TraceChannel` "TraceTypeQuery1" :`DrawTime` (`self.TraceCooldown`))
    ; reset trace cooldown
    (set `self.LastTrace` (`GameplayStatics.GetTimeSeconds`))
    ; Spawn NS and set Parameters
    (if true
      (bind _returnvalue_3 (`NiagaraFunctionLibrary.SpawnSystemAttached` "/Game/VFX/NS_electricbarrier.NS_electricbarrier" (`self.DefaultSceneRoot`) "None" (0.0 0.0 0.0) (struct) "SnapToTargetIncludingScale" true))
      (`NiagaraComponent.SetNiagaraVariableVec3` _returnvalue_3 "BeamStartPoint" _returnvalue)
      (`NiagaraComponent.SetNiagaraVariableVec3` _returnvalue_3 "BeamEndPoint" _returnvalue_2))))

(fn `UserConstructionScript`)