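; BP_zapparea is an actor that throws electric arcs from its center area onto nearby surfaces.
; Each Tick, Zappline traces a random direction between Startpoint and Zappradius, ignoring StaticMeshActors tagged "bound" gathered at BeginPlay.
; Hits spawn an attached NS_electricArcs Niagara system with beam endpoints set from the start offset and normal-offset impact point.
; The cooldown check and a circle-stepping downward-trace variant are disconnected and never run.
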(event `self.ReceiveBeginPlay`
  ; Liste der nicht gezappten Objekte
  (bind _outactors (`GameplayStatics.GetAllActorsOfClassWithTag` "/Script/Engine.StaticMeshActor" "bound"))
  (set `self.Notzapping` _outactors))

(event `self.ReceiveTick`
  (params (DeltaSeconds :type "Float (single-precision)"))
  (`self.zappline`))

(fn `UserConstructionScript`)

(fn `zappline`
  (locals (RandomDirection :type "Vector Structure" :default (0.0 0.0 0.0)) (ImpactOffset :type "Float (double-precision)" :default 1.0) (lastpoint :type "Vector Structure" :default (0.0 0.0 0.0)) (currentpoint :type "Vector Structure"))
  (bind _returnvalue (`self.K2_GetActorLocation`))
  (bind _returnvalue_2 (* (`local.RandomDirection`) (`self.startpoint`)))
  ; check circle
  ; tracing in the sphere
  (set `local.RandomDirection` (`KismetMathLibrary.RandomUnitVector`))
  (bind _outhit (`KismetSystemLibrary.LineTraceSingle` (+ _returnvalue _returnvalue_2) (+ (- _returnvalue (0.0 0.0 0.0)) (* (`local.RandomDirection`) (`self.Zappradius`))) "TraceTypeQuery1" false (`self.Notzapping`) "None" true (struct :`R` 1.0 :`A` 1.0) (struct :`G` 1.0 :`A` 1.0) (`self.TraceCooldown`)))
  ; reset trace cooldown
  (set `self.Stepsize` (`GameplayStatics.GetTimeSeconds`))
  (bind (_bblockinghit _binitialoverlap _time _distance _location _impactpoint _normal _impactnormal) (`GameplayStatics.BreakHitResult` _outhit))
  ; Spawn NS and set Parameters
  (if _bblockinghit
    (bind _returnvalue_3 (`NiagaraFunctionLibrary.SpawnSystemAttached` "/Game/VFX/NS_electricArcs.NS_electricArcs" (`self.DefaultSceneRoot`) "None" (0.0 0.0 0.0) (struct) "KeepRelativeOffset" true))
    (`NiagaraComponent.SetNiagaraVariableVec3` _returnvalue_3 "BeamStartPoint" _returnvalue_2)
    (`NiagaraComponent.SetNiagaraVariableVec3` _returnvalue_3 "BeamEndPoint" (+ _impactpoint (* _impactnormal (`local.ImpactOffset`))))))