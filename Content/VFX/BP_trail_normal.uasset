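; Slap trail effect Blueprint that adds a Niagara trail to its owning BP_Slap_Player.
; On BeginPlay it spawns the trail attached to the attack collision sphere, centered between two mesh sockets, aligned along them and sized to their distance, then pauses it.
; Bound slap events reset the system one tick after a slap starts and reinitialize it when the slap stops.
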(event `self.ReceiveBeginPlay`
  ; Init
  (bind _asbp_slap_player (cast `/Game/Player/Prof/BP_Slap_Player` (`self.GetOwner`)))
  (`self.SpawnParticleSystem` _asbp_slap_player)
  (`self.BindToSlap` _asbp_slap_player)
  (`NiagaraComponent.SetPaused` (`self.Trail`) true))

(event `SpawnParticleSystem`
  (params (Player :type "/Game/Player/Prof/BP_Slap_Player Object Reference"))
  (bind _mesh (`Character.Mesh` Player))
  (bind _returnvalue (`SceneComponent.GetSocketLocation` _mesh "vfx_trail_end"))
  (bind _returnvalue_2 (`SceneComponent.GetSocketLocation` _mesh "vfx_trail_start"))
  (bind _returnvalue_3 (- _returnvalue _returnvalue_2))
  ; Spawn Particle System
  (bind _returnvalue_4 (`NiagaraFunctionLibrary.SpawnSystemAttached` "/Game/VFX/NS_trail2.NS_trail2" (`/Game/Player/Prof/BP_Slap_Player.Col_AttackSphere` Player) "None" (/ (+ _returnvalue_2 _returnvalue) 2.0) (`KismetMathLibrary.MakeRotFromY` _returnvalue_3) "KeepWorldPosition"))
  (bind _output_get (set `self.Trail` _returnvalue_4))
  (`FXSystemComponent.SetFloatParameter` _output_get "trailwidth" (`KismetMathLibrary.VSize` _returnvalue_3)))

(event `BindToSlap`
  (params (Player :type "/Game/Player/Prof/BP_Slap_Player Object Reference"))
  ; Bind Slap Events
  (`|ExecutionSequence`
    (:`then_0`
      (add `/Game/Player/Prof/BP_Slap_Player.SlapStarted` Player (delegate `OnSlapStarted`)))
    (:`then_1`
      (add `/Game/Player/Prof/BP_Slap_Player.SlapStopped` Player (delegate `OnSlapStopped`)))))

(event `OnSlapStarted`
  ; Bind Slap Events
  (`KismetSystemLibrary.DelayUntilNextTick`)
  (`NiagaraComponent.ResetSystem` (`self.Trail`)))

(event `OnSlapStopped`
  ; Bind Slap Events
  (`NiagaraComponent.ReinitializeSystem` (`self.Trail`)))