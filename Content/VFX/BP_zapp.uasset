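; Electric zapper VFX actor that throws random lightning arcs at nearby surfaces and kill beams at given targets.
; On a cooldown, Tick traces in a random, downward-biased direction, ignoring "bound"-tagged static meshes, and spawns Niagara arcs on hits.
; Each tick it also spawns kill beams toward every valid KillTargets entry regardless of trace hits, resetting the arc cooldown.
; KillTargets is not populated within this Blueprint.
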(event `self.ReceiveBeginPlay`
  ; Liste der nicht gezappten Objekte
  (bind _outactors (`GameplayStatics.GetAllActorsOfClassWithTag` "/Script/Engine.StaticMeshActor" "bound"))
  (set `self.Notzapping` _outactors))

(event `self.ReceiveTick`
  (params (DeltaSeconds :type "Float (single-precision)"))
  (`self.UpdateTraces`)
  (if (`KismetArrayLibrary.Array_IsNotEmpty` (`self.KillTargets`))
    (`self.VFX_TraceTargets` (`self.KillTargets`))))

(fn `UpdateTraces`
  (locals (RandomDirection :type "Vector Structure" :default (0.0 0.0 0.0)) (ImpactOffset :type "Float (double-precision)" :default 1.0))
  (bind _returnvalue (`self.K2_GetActorLocation`))
  (bind _randomdirection (`local.RandomDirection`))
  ; check cooldown
  (if (>= (- (`GameplayStatics.GetTimeSeconds`) (`self.LastTrace`)) (`self.TraceCooldown`))
    ; tracing in the sphere
    (set `local.RandomDirection` (`KismetMathLibrary.RandomUnitVector`))
    (bind _outhit (`KismetSystemLibrary.LineTraceSingle` (+ _returnvalue (* _randomdirection (100.0 100.0 100.0))) (+ (- _returnvalue (0.0 0.0 1000.0)) (* (`local.RandomDirection`) (`self.MaxRadius`))) "TraceTypeQuery1" false (`self.Notzapping`) "None" true (struct :`R` 1.0 :`A` 1.0) (struct :`G` 1.0 :`A` 1.0) (`self.TraceCooldown`)))
    ; reset trace cooldown
    (set `self.LastTrace` (`GameplayStatics.GetTimeSeconds`))
    (bind (_bblockinghit _binitialoverlap _time _distance _location _impactpoint _normal _impactnormal) (`GameplayStatics.BreakHitResult` _outhit))
    ; Spawn NS and set Parameters
    (if _bblockinghit
      (bind _returnvalue_2 (`NiagaraFunctionLibrary.SpawnSystemAttached` "/Game/VFX/NS_electricArcs.NS_electricArcs" (`self.DefaultSceneRoot`) "None" (0.0 0.0 0.0) (struct) "KeepRelativeOffset" true))
      (`NiagaraComponent.SetNiagaraVariableVec3` _returnvalue_2 "BeamStartPoint" (* _randomdirection (`self.MinRadius`)))
      (`NiagaraComponent.SetNiagaraVariableVec3` _returnvalue_2 "BeamEndPoint" (+ _impactpoint (* _impactnormal (`local.ImpactOffset`))))
      (`NiagaraComponent.SetNiagaraVariableVec3` _returnvalue_2 "ImpactNormal" _impactnormal))))

(fn `UserConstructionScript`)

(fn `VFX_TraceTargets`
  (params (Targets :type "Array of Actor Object Reference"))
  (locals (RandomDirection :type "Vector Structure" :default (0.0 0.0 0.0)) (ImpactOffset :type "Float (double-precision)" :default 1.0))
  (bind _returnvalue (* (`local.RandomDirection`) (`self.MinRadius`)))
  (for _array_element Targets
    (if (`KismetSystemLibrary.IsValid` _array_element)
      (bind _returnvalue_2 (`SceneComponent.K2_GetComponentLocation` (`self.GetComponentByClass` _array_element "/Script/Engine.MeshComponent")))
      (bind _outhit (`KismetSystemLibrary.LineTraceSingle` :`Start` (+ (`self.K2_GetActorLocation`) _returnvalue) :`End` _returnvalue_2 :`TraceChannel` "TraceTypeQuery1" :`DrawTime` (`self.TraceCooldown`)))
      ; reset trace cooldown
      (set `self.LastTrace` (`GameplayStatics.GetTimeSeconds`))
      ; Spawn NS and set Parameters
      (bind _returnvalue_3 (`NiagaraFunctionLibrary.SpawnSystemAttached` "/Game/VFX/NS_electrickill.NS_electrickill" (`self.DefaultSceneRoot`) "None" (0.0 0.0 0.0) (struct) "KeepRelativeOffset" true))
      (`NiagaraComponent.SetNiagaraVariableVec3` _returnvalue_3 "BeamStartPoint" _returnvalue)
      (`NiagaraComponent.SetNiagaraVariableVec3` _returnvalue_3 "BeamEndPoint" (+ _returnvalue_2 (0.0 0.0 100.0)))
      (`NiagaraComponent.SetNiagaraVariableVec3` _returnvalue_3 "ImpactNormal" (`.ImpactNormal` (`GameplayStatics.BreakHitResult` _outhit))))))