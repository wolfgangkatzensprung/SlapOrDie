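; BP_CamLocator is a camera locator with a sphere volume that reports a weight based on player proximity.
; GetCurrentWeight takes the first overlapping BP_Slap_Player (marked temporary) and scales linearly from one at the sphere's center to zero at its radius, returning zero when none overlap.
; Logic for tracking players inside and signaling activation or deactivation is disconnected, leaving both overlap events empty.
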(event `self.Col_Sphere.OnComponentBeginOverlap`
  (params (OverlappedComponent :type "PrimitiveComponent Object Reference") (OtherActor :type "Actor Object Reference") (OtherComp :type "PrimitiveComponent Object Reference") (OtherBodyIndex :type Integer) (bFromSweep :type Boolean) (SweepResult :type "HitResult Structure (by ref)")))

(event `self.Col_Sphere.OnComponentEndOverlap`
  (params (OverlappedComponent :type "PrimitiveComponent Object Reference") (OtherActor :type "Actor Object Reference") (OtherComp :type "PrimitiveComponent Object Reference") (OtherBodyIndex :type Integer)))

(fn `GetCurrentWeight`
  (returns (Weight :type "Float (double-precision)"))
  (bind _overlappingactors (`self.GetOverlappingActors` "/Game/Player/Prof/BP_Slap_Player.BP_Slap_Player_C"))
  (bind _col_sphere (`self.Col_Sphere`))
  (if (`KismetArrayLibrary.Array_IsEmpty` _overlappingactors)
    (return 0.0)
    (else
      (return (`|EaseFunction` "Linear" (- 1.0 (/ (`KismetMathLibrary.Vector_Distance` (`SceneComponent.K2_GetComponentLocation` (`Actor.RootComponent` (`|GetArrayItem` _overlappingactors))) (`SceneComponent.K2_GetComponentLocation` _col_sphere)) (`SphereComponent.SphereRadius` _col_sphere))) 0.0 1.0)))))

(fn `UserConstructionScript`)