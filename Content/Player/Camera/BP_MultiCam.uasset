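; Shared multiplayer camera that frames all alive players and becomes the local controller's view target.
; Each tick it targets the weighted average of player mesh positions and BP_CamLocator points, smoothed, clamped within location confines and flattened to Z zero.
; Boom length follows the spread between players through an ease-out curve with interpolation.
; With one player state, positioning bypasses this and snaps to that player's mesh.
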(event `OnLocatorDeactivated`
  (params (Locator :type "/Game/Player/Camera/BP_CamLocator Object Reference"))
  ; Initialize Locator Bindings
  (`BlueprintSetLibrary.Set_Remove` (`self.ActiveLocators`) Locator))

(event `OnLocatorActivated`
  (params (Locator :type "/Game/Player/Camera/BP_CamLocator Object Reference"))
  ; Initialize Locator Bindings
  (`BlueprintSetLibrary.Set_Add` (`self.ActiveLocators`) Locator))

(event `self.ReceiveBeginPlay`
  (`|ExecutionSequence`
    (:`then_0`
      ; Initialize Locator Bindings
      (bind _outactors (`GameplayStatics.GetAllActorsOfClass` "/Game/Player/Camera/BP_CamLocator.BP_CamLocator_C"))
      (for _array_element _outactors
        (add `/Game/Player/Camera/BP_CamLocator.LocatorActivated` _array_element (delegate `OnLocatorActivated`))
        (add `/Game/Player/Camera/BP_CamLocator.LocatorDeactivated` _array_element (delegate `OnLocatorDeactivated`))))
    (:`then_1`
      ; Cam Start Location is Player Location
      (bind _output_get (set `self.LastCamLocation` (`SceneComponent.K2_GetComponentLocation` (`Character.Mesh` (`GameplayStatics.GetPlayerCharacter` 0)))))
      (`self.ApplyCameraLocation` _output_get 123.0))
    (:`then_2`
      (`self.TryInitializeCam`))))

(event `self.ReceiveTick`
  (params (DeltaSeconds :type "Float (single-precision)"))
  ; Tick
  (`self.MoveCam`))

(fn `ApplyCameraLocation`
  (params (TargetLocation :type "Vector Structure") (InterpolationSpeed :type "Float (double-precision)"))
  (bind _returnvalue (`KismetMathLibrary.MakeVector` (.x (`KismetMathLibrary.ClampVectorSize` (`KismetMathLibrary.VInterpTo` (`self.LastCamLocation`) TargetLocation (`GameplayStatics.GetWorldDeltaSeconds`) InterpolationSpeed) (.x (`self.LocationConfinesMinMax`)) (.y (`self.LocationConfinesMinMax`)))) (.y (`KismetMathLibrary.ClampVectorSize` (`KismetMathLibrary.VInterpTo` (`self.LastCamLocation`) TargetLocation (`GameplayStatics.GetWorldDeltaSeconds`) InterpolationSpeed) (.x (`self.LocationConfinesMinMax`)) (.y (`self.LocationConfinesMinMax`))))))
  (if (> (`GameplayStatics.GetNumPlayerStates`) 1)
    (`SceneComponent.K2_SetWorldLocation` (`self.CameraBoom`) _returnvalue false false)
    (bind _output_get (set `self.LastCamLocation` _returnvalue))
    (`KismetSystemLibrary.PrintString` (`KismetStringLibrary.Conv_VectorToString` _output_get) true true (struct :`R` 1.0 :`G` 0.944197 :`B` 0.182375 :`A` 1.0) 2.0 "caml")
    (else
      ; 1 Player bypass cam logic
      (bind _returnvalue_2 (`GameplayStatics.GetActorOfClass` "/Game/Player/Prof/BP_Slap_Player.BP_Slap_Player_C"))
      (`SceneComponent.K2_SetWorldLocation` (`self.CameraBoom`) (`SceneComponent.K2_GetComponentLocation` (`Character.Mesh` _returnvalue_2)) false false))))

(fn `ApplyCameraZoom`
  (params (TargetZoom :type "Float (double-precision)"))
  (bind _output_get (set `SpringArmComponent.TargetArmLength` (`KismetMathLibrary.FMin` (`KismetMathLibrary.FInterpTo` (`self.LastCamZoom`) TargetZoom (`GameplayStatics.GetWorldDeltaSeconds`) (`self.CamSmoothingInterpolationSpeed`)) (`self.MaxCamZoom`)) (`self.CameraBoom`)))
  (set `self.LastCamZoom` _output_get))

(fn `CalculateHighestDistance`
  (params (OwnCharacter :type "Character Object Reference") (AlivePlayers :type "Array of /Game/Player/Prof/BP_Slap_Player Object Reference") (CurrentHighestDistance :type "Float (double-precision)"))
  (returns (HighestDistance :type "Float (double-precision)"))
  (for _array_element AlivePlayers
    (if (`KismetSystemLibrary.IsValid` _array_element)
      (bind _returnvalue (`KismetMathLibrary.Vector_Distance` (`SceneComponent.K2_GetComponentLocation` (`Character.Mesh` _array_element)) (`SceneComponent.K2_GetComponentLocation` (`Character.Mesh` OwnCharacter))))
      (if (> _returnvalue CurrentHighestDistance)
        (return _returnvalue)))))

(fn `CalculateTargetPosition`
  (params (PlayerWorldLocationsSum :type "Vector Structure") (TotalWeight :type "Float (double-precision)"))
  (returns (TargetPos :type "Vector Structure"))
  (locals (TotalWorldLocationSum :type "Vector Structure"))
  (bind _outactors (`GameplayStatics.GetAllActorsOfClass` "/Game/Player/Camera/BP_CamLocator.BP_CamLocator_C"))
  (for _array_element _outactors
    (bind _weight (`/Game/Player/Camera/BP_CamLocator.GetCurrentWeight` _array_element))
    (set `local.TotalWorldLocationSum` (+ (`local.TotalWorldLocationSum`) (* (`SceneComponent.K2_GetComponentLocation` (`/Game/Player/Camera/BP_CamLocator.Col_Sphere` _array_element)) _weight))))
  (return (/ (+ (`local.TotalWorldLocationSum`) PlayerWorldLocationsSum) TotalWeight)))

(fn `CalculateTotalWeight`
  (params (CurrentAlivePlayerAmount :type Integer))
  (returns (Weight :type "Float (double-precision)"))
  (locals (CurrentWeight :type "Float (double-precision)"))
  (bind _outactors (`GameplayStatics.GetAllActorsOfClass` "/Game/Player/Camera/BP_CamLocator.BP_CamLocator_C"))
  (for _array_element _outactors
    (bind _weight (`/Game/Player/Camera/BP_CamLocator.GetCurrentWeight` _array_element))
    (set `local.CurrentWeight` (+ _weight (`local.CurrentWeight`))))
  (return (+ (`KismetMathLibrary.Conv_IntToDouble` CurrentAlivePlayerAmount) (`local.CurrentWeight`))))

(fn `CalculateZoom`
  (params (HighestDistance :type "Float (double-precision)"))
  (returns (Zoom :type "Float (double-precision)"))
  (return (`KismetMathLibrary.FMax` (`|EaseFunction` "EaseOut" (/ (- HighestDistance (`self.ZoomDistanceThreshold`)) (- (`self.MaxCamZoom`) (`self.MinCamZoom`))) (`self.MinCamZoom`) (`self.MaxCamZoom`)) (`self.MinCamZoom`))))

(fn `InitializeFromPlayer`
  (params (PlayerController :type "PlayerController Object Reference"))
  (`/Engine/EditorBlueprintResources/StandardMacros.IsValid` PlayerController
    (:`Is Valid`
      (`PlayerController.SetViewTargetWithBlend` PlayerController self 1.0 "VTBlend_Linear" 0.0 false))))

(fn `MoveCam`
  (locals (WorldLocationSum :type "Vector Structure" :default (0.0 0.0 0.0)) (CurrentAlivePlayers :type Integer) (AlivePlayers :type "Array of /Game/Player/Prof/BP_Slap_Player Object Reference") (HighestDistance :type "Float (double-precision)"))
  ; Get Players from Game State
  (bind _asgs_slap_state (cast `/Game/Slappedy/GS_SlapState` (`GameplayStatics.GetGameState`)))
  (bind _output_get (set `local.AlivePlayers` (`/Game/Slappedy/GS_SlapState.AlivePlayers` _asgs_slap_state)))
  ; Loop through Players
  (if (`KismetArrayLibrary.Array_IsNotEmpty` _output_get)
    (for _array_element _output_get
      (if (`KismetSystemLibrary.IsValid` _array_element)
        ; Add up Player World Locations
        (set `local.WorldLocationSum` (+ (`SceneComponent.K2_GetComponentLocation` (`Character.Mesh` _array_element)) (`local.WorldLocationSum`)))
        ; Find Highest Distance between Players
        (bind _highestdistance (`self.CalculateHighestDistance` _array_element (`local.AlivePlayers`) (`local.HighestDistance`)))
        (bind _output_get_2 (set `local.HighestDistance` _highestdistance))))
    (bind _weight (`self.CalculateTotalWeight` (`KismetArrayLibrary.Array_Length` _output_get)))
    (bind _targetpos (`self.CalculateTargetPosition` (`local.WorldLocationSum`) _weight))
    ; Apply Camera Position
    (`self.ApplyCameraLocation` _targetpos (`self.CamSmoothingInterpolationSpeed`))
    ; Zoom out to keep Players in view
    (bind _zoom (`self.CalculateZoom` _output_get_2))
    (`self.ApplyCameraZoom` _zoom)))

(fn `TryInitializeCam`
  (returns (InitSucceeded :type Boolean))
  (bind _outactors (`GameplayStatics.GetAllActorsOfClass` "/Game/Player/BP_PlayerController.BP_PlayerController_C"))
  (for _array_element _outactors
    (if (`Controller.IsLocalPlayerController` _array_element)
      (`PlayerController.SetViewTargetWithBlend` _array_element self 1.0 "VTBlend_Linear" 0.0 false)
      (return true)))
  (return false))

(fn `UserConstructionScript`)