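; Player controller for the Slap game, handling possession, pause toggling and networked lobby UI.
; Possession flags BP_Slap_Player as possessed, BeginPlay locks input to UI, and pause uses a DoOnce reset two ticks later.
; Server events forward ready toggles to GM_Lobby and relay HUD updates through multicasts, retrying each tick until the lobby widget exists.
; Also fades into end music as a workaround and prints controller IDs every tick.
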(event `self.ReceiveTick`
  (params (DeltaSeconds :type "Float (single-precision)"))
  (`KismetSystemLibrary.PrintString` (`KismetTextLibrary.Conv_TextToString` (`|FormatText` "{i} use Controller ID {id}" self (`GameplayStatics.GetPlayerControllerID` self))) true true (struct :`R` 0.485771 :`G` 0.940169 :`B` 1.0 :`A` 1.0) 1.0 (`KismetStringLibrary.Conv_StringToName` (`KismetGuidLibrary.Conv_GuidToString` (`self.ActorGuid`)))))

(event `self.ReceivePossess`
  (params (PossessedPawn :type "Pawn Object Reference"))
  ; On Possess
  (`KismetSystemLibrary.DelayUntilNextTick`)
  (bind _asbp_slap_player (cast `/Game/Player/Prof/BP_Slap_Player` PossessedPawn))
  (set `/Game/Player/Prof/BP_Slap_Player.IsPossessed` true _asbp_slap_player))

(event `self.ReceiveBeginPlay`
  ; Wait for match Start
  (`WidgetBlueprintLibrary.SetInputMode_UIOnlyEx` self null "DoNotLock" true))

(event `EnhancedInput|/Game/Player/Input/IA_Pause`
  (params (ActionValue :type Boolean) (ElapsedSeconds :type "Float (double-precision)") (TriggeredSeconds :type "Float (double-precision)") (InputAction :type "InputAction Object Reference" :default "/Game/Player/Input/IA_Pause.IA_Pause"))
  (bind _pausewidget (`/Game/Slappedy/HUD_Slap.PauseWidget` (cast `/Game/Slappedy/HUD_Slap` (`self.GetHUD` (`GameplayStatics.GetPlayerController` 0)) :!pure true)))
  ;[0.06511 0.141 0.15 0.5] Pause Input
  (:`Started`
    (`/Engine/EditorBlueprintResources/StandardMacros.DoOnce` false :!label _label
      (:`Completed`
        (if (`Widget.IsVisible` _pausewidget)
          (`/Game/Menu/UI_Menu/WBP_Pause.HideAndContinue` _pausewidget)
          (else
            (`/Game/Menu/UI_Menu/WBP_Pause.ShowAndPause` _pausewidget)))
        (`KismetSystemLibrary.DelayUntilNextTick`)
        (`KismetSystemLibrary.DelayUntilNextTick`)
        (`self.ResetPauseInput`)))))

(event `ResetPauseInput`
  ;[0.06511 0.141 0.15 0.5] Pause Input
  (goto _label :!via `Reset`))

(event `PlayEndMusic`
  (bind _asgi_slap_instance (cast `/Game/Slappedy/GI_SlapInstance` (`GameplayStatics.GetGameInstance`) :!pure true))
  ; End Music Workaround
  (`/Game/Slappedy/GI_SlapInstance.FadeOutMusic` _asgi_slap_instance 1.0)
  (`KismetSystemLibrary.Delay` 1.0)
  (`/Game/Slappedy/GI_SlapInstance.PlayMusicDirectly` _asgi_slap_instance "End"))

(event `Server_TogglePlayerReady`
  (params (PlayerNumber :type Integer))
  ;[0.15 0.1484 0.04978 0.5] UI - Lobby
  ;; Notify Server - Player has readied
  (bind _asgm_lobby (cast `/Game/Menu/GM_Lobby` (`GameplayStatics.GetGameMode`)))
  (`/Game/Menu/GM_Lobby.TogglePlayerReady` _asgm_lobby PlayerNumber))

(event `Server_UpdatePlayerIcons`
  ;[0.15 0.1484 0.04978 0.5] UI - Lobby
  (`self.MC_UpdatePlayerIcons`))

(event `MC_UpdatePlayerIcons`
  (bind _lobbywidget (`/Game/Slappedy/HUD_Slap.LobbyWidget` (cast `/Game/Slappedy/HUD_Slap` (`self.GetHUD`) :!pure true)))
  ;[0.15 0.1484 0.04978 0.5] UI - Lobby
  ;; Update Players in Lobby
  (`KismetSystemLibrary.DelayUntilNextTick` :!label _label_2)
  (`/Engine/EditorBlueprintResources/StandardMacros.IsValid` _lobbywidget
    (:`Is Valid`
      (`/Game/Menu/UI_Menu/WBP_Lobby.UpdatePlayerIcons` _lobbywidget))
    (:`Is Not Valid`
      (goto _label_2))))

(event `Server_UpdateReadyUI`
  (params (PlayersReady :type "Array of Boolean"))
  ;[0.15 0.1484 0.04978 0.5] UI - Lobby
  ;; Update Ready States
  (`self.MC_UpdateReadyUI` PlayersReady))

(event `MC_UpdateReadyUI`
  (params (PlayersReady :type "Array of Boolean"))
  (bind _lobbywidget (`/Game/Slappedy/HUD_Slap.LobbyWidget` (cast `/Game/Slappedy/HUD_Slap` (`self.GetHUD`) :!pure true)))
  ;[0.15 0.1484 0.04978 0.5] UI - Lobby
  ;; Update Ready States
  (if (== self (`GameplayStatics.GetPlayerController` 0))
    (`KismetSystemLibrary.DelayUntilNextTick` :!label _label_3)
    (`/Engine/EditorBlueprintResources/StandardMacros.IsValid` _lobbywidget
      (:`Is Valid`
        (`/Game/Menu/UI_Menu/WBP_Lobby.UpdatePlayersReady` _lobbywidget PlayersReady))
      (:`Is Not Valid`
        (goto _label_3)))))

(event `Server_FinishLoadingScreen`
  (`self.MC_FinishLoadingScreen`))

(event `MC_FinishLoadingScreen`
  (`KismetSystemLibrary.DelayUntilNextTick`)
  (`/Game/Slappedy/HUD_Slap.FinishLoadingScreen` (cast `/Game/Slappedy/HUD_Slap` (`self.GetHUD`) :!pure true)))

(fn `UserConstructionScript`)