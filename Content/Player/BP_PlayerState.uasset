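; Player state for the slap game, holding each player's data, ready flag, score and score multiplier.
; Server events set or reset PlayerData, CopyProperties carries it across player states, and its RepNotify updates player icons and the game instance.
; Kills from not-yet-used trap IDs raise the multiplier a tick later until LoseMultiplier resets both, and its RepNotify updates the pawn's text.
; Tick prints PlayerData for debugging.
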(event `self.ReceiveTick`
  (params (DeltaSeconds :type "Float (single-precision)"))
  (bind (_playerdata_playername _playerdata_playercontroller _playerdata_playernumber _playerdata_color _playerdata_connected) (break `/Game/Slappedy/Struct_PlayerData` (`self.PlayerData`)))
  ; Debug Info
  (`KismetSystemLibrary.PrintString` (`KismetTextLibrary.Conv_TextToString` (`|FormatText` "PlayerData: {n}, {pc}, {num}, {col}, {con}" _playerdata_playername _playerdata_playercontroller _playerdata_playernumber _playerdata_color _playerdata_connected)) true true (struct :`R` 0.893823 :`G` 1.0 :`A` 1.0) 1.0 (`KismetStringLibrary.Conv_StringToName` (`KismetStringLibrary.Conv_ObjectToString` self))))

(event `Server_SetReadyToSlap`
  ; Level is loaded and Player is ready
  (set `self.ReadyToSlap` true))

(event `Server_InitState`
  (params (PlayerData :type "/Game/Slappedy/Struct_PlayerData Structure"))
  ; Init
  (set `self.PlayerData` PlayerData))

(event `self.ReceiveCopyProperties`
  (params (NewPlayerState :type "PlayerState Object Reference"))
  ; Persistent PlayerData
  (bind _asbp_player_state (cast `/Game/Player/BP_PlayerState` NewPlayerState))
  (set `/Game/Player/BP_PlayerState.PlayerData` (`self.PlayerData`) _asbp_player_state))

(event `Server_ResetPlayerData`
  (set `self.PlayerData` (make `/Game/Slappedy/Struct_PlayerData` "NoName" null)))

(event `AddMultiplier`
  (`KismetSystemLibrary.DelayUntilNextTick`)
  (set `self.Multiplier` (+ (`self.Multiplier`) 0.2)))

(fn `AddScore`
  (params (AddScore :type Integer))
  (set `self.PlayerScore` (`KismetMathLibrary.FTrunc` (`KismetMathLibrary.Conv_IntToDouble` (+ (* AddScore (`self.Multiplier`)) (`self.PlayerScore`))))))

(fn `GetPlayerNumber`
  (returns (PlayerNumber :type Integer))
  (return (`.PlayerNumber_8_D9780B4E45446C2C095DA69A3B2DACF9` (break `/Game/Slappedy/Struct_PlayerData` (`self.PlayerData`)))))

(fn `LoseMultiplier`
  ; Reset Multiplier and Used Traps
  (set `self.Multiplier` 1.0)
  (set `self.UsedTrapIds` (`|MakeSet` "")))

(fn `OnEnemyKill`
  (params (TrapId :type String))
  (if (not (`BlueprintSetLibrary.Set_Contains` (`self.UsedTrapIds`) TrapId))
    (`BlueprintSetLibrary.Set_Add` (`self.UsedTrapIds`) TrapId)
    (`self.AddMultiplier`)))

(fn `OnPlayerDataAdded`
  (bind _asbp_player_controller (cast `/Game/Player/BP_PlayerController` (`GameplayStatics.GetPlayerController` 0)))
  (`/Game/Player/BP_PlayerController.MC_UpdatePlayerIcons` _asbp_player_controller)
  (bind _asgi_slap_instance (cast `/Game/Slappedy/GI_SlapInstance` (`GameplayStatics.GetGameInstance`)))
  (`/Game/Slappedy/GI_SlapInstance.AddPlayerData` _asgi_slap_instance (`self.PlayerData`)))

(fn `OnRep_Multiplier`
  (bind _asbp_slap_player (cast `/Game/Player/Prof/BP_Slap_Player` (`self.PawnPrivate`)))
  (`/Game/Player/Prof/BP_Slap_Player.UpdateMultiplierText` _asbp_slap_player (`self.Multiplier`)))

(fn `OnRep_PlayerData`
  (bind (_playerdata_playername _playerdata_playercontroller _playerdata_playernumber) (break `/Game/Slappedy/Struct_PlayerData` (`self.PlayerData`)))
  (if (!= _playerdata_playernumber 0)
    (`self.OnPlayerDataAdded`)))

(fn `UserConstructionScript`)