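; Game mode for a co-op slap match that runs a kill-target round against enemies spawned from portals.
; Kill target, enemy cap and spawn delay scale with difficulty and player count from GI_SlapInstance.
; Once all players are ready it starts a countdown, then loops triggering random idle spawn points below the cap.
; It kicks late logins and pushes alive players and kill progress to GS_SlapState, ending the match at the target.
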(event Custom|Start%20Match
  ;[0.15 0.15 0.15 0.5] Start Match
  (Utilities|FlowControl|Delay 1.0)
  (bind _outactors (Actor|GetAllActorsOfClass "/Game/Player/Prof/BP_Slap_Player.BP_Slap_Player_C"))
  (for _array_element _outactors
    (Default|ServerStartCountdown _array_element))
  (Utilities|FlowControl|Delay 4.0) ; ToDo: Callback statt Delay, sonst ist man bei starkem lag noch im countdown
  (CallFunction|StartGameSpawnLoopRoutine)
  (bind _outactors_2 (Actor|GetAllActorsOfClass "/Game/Player/Prof/BP_Slap_Player.BP_Slap_Player_C"))
  (for _array_element_2 _outactors_2
    (Default|MConMatchStarted _array_element_2)))

(event Custom|StartGameSpawnLoopRoutine
  ;[0.15 0.15 0.15 0.5] Enemy Spawning
  (if (Variables|Default|GetMatchIsRunning) :!label _label
    (bind _outactors (Actor|GetAllActorsOfClass "/Game/Enemy/BP_Enemy_Base.BP_Enemy_Base_C"))
    (if (< (Utilities|Array|Length _outactors) (Variables|Default|GetMaxEnemiesCount)) ; can spawn enemies
      (CallFunction|TriggerPortal)
      (Utilities|FlowControl|Delay (Variables|Default|GetCurrentSpawnDelay))
      (goto _label)
      (else
        _)))
  (Utilities|FlowControl|Delay 0.5)
  (goto _label))

(event Custom|TriggerPortal
  ;[0.15 0.15 0.15 0.5] Enemy Spawning
  (bind _spawnpoint (CallFunction|GetRandomEnemySpawnPoint))
  (if (Variables|/Game/Enemy/EnemyPortal/BP_EnemySpawnPoint.BP_EnemySpawnPoint_C|GetIsSpawning _spawnpoint) ; already spawning?
    (Utilities|FlowControl|Delay 0.1)
    (Utilities|FlowControl|DelayUntilNextTick)
    (CallFunction|TriggerPortal) ; try again
    (else
      (Default|StartSpawnRoutine _spawnpoint))))

(event EventOnSetMatchState
  (params (NewState :type Name :default "None"))
  ;[0.15 0.15 0.15 0.5] End Match
  (switch name NewState
    (:WaitingPostMatch
      (Utilities|Time|SetGlobalTimeDilation 0.25)
      (Utilities|FlowControl|Delay 0.5)
      (Utilities|Time|SetGlobalTimeDilation 1.0)
      (bind _asgs_slap_state (Utilities|Casting|CastToGS_SlapState (Game|GetGameState)))
      (Default|ServerMatchEnded _asgs_slap_state))))

(event EventPostLogin
  (params (NewPlayer :type Player%20Controller%20Object%20Reference))
  ;[0.15 0.15 0.15 0.5] Disallow Join after Lobby
  (Class|AdvancedSessionsLibrary|KickPlayer NewPlayer "Match is already running!")
  (Development|PrintString "Someone tried Login during Match but was instakicked!"))

(event EventBeginPlay
  ;[0.15 0.15 0.15 0.5] Init
  (CallFunction|InitEnemyTargetKillsAmount)
  (CallFunction|InitEnemyCap)
  (CallFunction|InitSpawnRate)
  (CallFunction|InitSpawnLocations)
  (Utilities|FlowControl|Delay 5.0)
  ;[0.15 0.15 0.15 0.5] Check Players ready, dann start match
  (bind _allready (CallFunction|AreAllPlayersReady :!label _label))
  (if _allready
    (Utilities|FlowControl|Delay 1.0)
    (CallFunction|SetMaxKills (Variables|Default|GetMaxKillsProgress))
    (CallFunction|FinishLoadingScreen)
    (Utilities|FlowControl|Delay 1.0)
    (Variables|Default|SetMatchIsRunning true)
    (CallFunction|StartMatch)
    (else
      (Development|PrintString "Waiting for Players..." true true "(R=0.000000,G=0.660000,B=1.000000,A=1.000000)" 2.0 "wait")
      (Utilities|FlowControl|DelayUntilNextTick)
      (goto _label))))

(fn ConstructionScript)

(fn GetAlivePlayers
  (bind _result (Utilities|Set|ToArray (Variables|Default|GetAlivePlayers)))
  (return _result))

(fn GetRandomPlayer
  (bind _playersalive (CallFunction|GetAlivePlayers))
  (return (Utilities|Array|Get(acopy) _playersalive (Math|Random|RandomIntegerinRange 0 (Utilities|Array|Length _playersalive)))))

(fn OnPlayerSpawned
  (params (Player :type BP%20Slap%20Player%20Object%20Reference))
  (bind _aliveplayers (Variables|Default|GetAlivePlayers))
  (Utilities|Set|Add _aliveplayers Player)
  (CallFunction|UpdateGameStateAlivePlayers _aliveplayers))

(fn OnPlayerDied
  (params (PlayerWhoDied :type BP%20Slap%20Player%20Object%20Reference%20%28by%20ref%29))
  (bind _aliveplayers (Variables|Default|GetAlivePlayers))
  (Utilities|Set|Remove _aliveplayers PlayerWhoDied)
  (CallFunction|UpdateGameStateAlivePlayers _aliveplayers))

(fn OnEnemyDeath
  (bind _result (Math|Integer|IncrementInt (Variables|Default|GetKillsProgress))
    (:%20%20
      (CallFunction|UpdateGameStateProgress)
      (if (>= _result (Variables|Default|GetMaxKillsProgress))
        (Class|GameMode|EndMatch)))))

(fn UpdateGameStateAlivePlayers
  (params (A :type Set%20of%20BP%20Slap%20Player%20Object%20References))
  (bind _asgs_slap_state (Utilities|Casting|CastToGS_SlapState (Game|GetGameState)))
  (bind _result (Utilities|Set|ToArray A))
  (Default|ServerAlivePlayersChanged _asgs_slap_state _result))

(fn UpdateGameStateProgress
  (bind _asgs_slap_state (Utilities|Casting|CastToGS_SlapState (Game|GetGameState)))
  ;[0.15 0.15 0.15 0.5] Update RepVars in GameState
  (Variables|/Game/Slappedy/GS_SlapState.GS_SlapState_C|SetProgressPercent _asgs_slap_state (/ (Variables|Default|GetKillsProgress) (Math|Conversions|ToFloat(Integer) (Variables|Default|GetMaxKillsProgress))))
  (Variables|/Game/Slappedy/GS_SlapState.GS_SlapState_C|SetKillsProgress _asgs_slap_state (Variables|Default|GetKillsProgress))
  (Variables|/Game/Slappedy/GS_SlapState.GS_SlapState_C|SetMaxKillsProgress _asgs_slap_state (Variables|Default|GetMaxKillsProgress)))

(fn AreAllPlayersReady
  (bind _outactors (Actor|GetAllActorsOfClass "/Game/Player/BP_PlayerState.BP_PlayerState_C"))
  (bind _asgi_slap_instance (Utilities|Casting|CastToGI_SlapInstance (Game|GetGameInstance)))
  (if (>= (Utilities|Array|Length _outactors) (Variables|/Game/Slappedy/GI_SlapInstance.GI_SlapInstance_C|GetPlayerAmount _asgi_slap_instance))
    (for _array_element _outactors
      (if (.connected (Variables|/Game/Player/BP_PlayerState.BP_PlayerState_C|GetPlayerData _array_element))
        (if (not (Variables|/Game/Player/BP_PlayerState.BP_PlayerState_C|GetReadyToSlap _array_element))
          (LocalVariables|SetRetVal false))))
    (return (LocalVariables|GetRetVal))
    (else
      (return false))))

(fn InitSpawnLocations
  (bind _outactors (Actor|GetAllActorsOfClass "/Game/Enemy/EnemyPortal/BP_EnemySpawnPoint.BP_EnemySpawnPoint_C"))
  (for _array_element _outactors
    (Utilities|Set|Add (Variables|Default|GetEnemySpawnPoints) _array_element)))

(fn GetRandomEnemySpawnPoint
  (bind _result (Utilities|Set|ToArray (Variables|Default|GetEnemySpawnPoints)))
  (return (Utilities|Array|Get(acopy) _result (Math|Random|RandomIntegerinRange 0 (- (Utilities|Set|Length (Variables|Default|GetEnemySpawnPoints)) 1)))))

(fn ResetMatch
  (Variables|Default|SetMatchIsRunning false)
  (bind _outactors (Actor|GetAllActorsOfClass "/Game/Player/Prof/BP_Slap_Player.BP_Slap_Player_C"))
  (bind _outactors_2 (Actor|GetAllActorsOfClass "/Script/Engine.PlayerStart"))
  (for (_array_element _array_index) _outactors
    (Transformation|Teleport _array_element (.location (Transformation|GetActorTransform (Utilities|Array|Get(acopy) _outactors_2 _array_index))) (.rotation (Transformation|GetActorTransform (Utilities|Array|Get(acopy) _outactors_2 _array_index))))))

(fn SetMaxKills
  (params (MaxKillsProgress :type Integer))
  (Variables|Default|SetMaxKillsProgress MaxKillsProgress)
  (CallFunction|UpdateGameStateProgress))

(fn FinishLoadingScreen
  (bind _outactors (Actor|GetAllActorsOfClass "/Game/Player/BP_PlayerController.BP_PlayerController_C"))
  (for _array_element _outactors
    (Default|ServerFinishLoadingScreen _array_element)))

(fn InitSpawnRate
  (Variables|Default|SetCurrentSpawnDelay (Math|Float|MapRangeClamped (Variables|/Game/Slappedy/GI_SlapInstance.GI_SlapInstance_C|GetDifficulty (.AsGI%20Slap%20Instance (Utilities|Casting|CastToGI_SlapInstance (Game|GetGameInstance)))) 0.1 1.0 (Variables|Default|GetMaxDelayBetweenSpawns) (Variables|Default|GetMinDelay%20Between%20Spawns))))

(fn InitEnemyCap
  (bind _returnvalue (Game|GetGameInstance))
  (bind _asgi_slap_instance (Utilities|Casting|CastToGI_SlapInstance _returnvalue))
  (bind _difficulty (Variables|/Game/Slappedy/GI_SlapInstance.GI_SlapInstance_C|GetDifficulty _asgi_slap_instance))
  (switch int (Variables|/Game/Slappedy/GI_SlapInstance.GI_SlapInstance_C|GetPlayerAmount _asgi_slap_instance)
    (:1
      (Variables|Default|SetMaxEnemiesCount (Math|Float|Truncate (Math|Float|MapRangeClamped _difficulty 0.1 1.0 1.0 2e+01))))
    (:2
      (Variables|Default|SetMaxEnemiesCount (Math|Float|Truncate (Math|Float|MapRangeClamped _difficulty 0.1 1.0 1.0 2e+01))))
    (:3
      (Variables|Default|SetMaxEnemiesCount (Math|Float|Truncate (Math|Float|MapRangeClamped _difficulty 0.1 1.0 2.0 2e+01))))
    (:4
      (Variables|Default|SetMaxEnemiesCount (Math|Float|Truncate (Math|Float|MapRangeClamped _difficulty 0.1 1.0 2.0 2e+01))))))

(fn InitEnemyTargetKillsAmount
  (bind _returnvalue (Game|GetGameInstance))
  (bind _asgi_slap_instance (Utilities|Casting|CastToGI_SlapInstance _returnvalue))
  (bind _difficulty (Variables|/Game/Slappedy/GI_SlapInstance.GI_SlapInstance_C|GetDifficulty _asgi_slap_instance))
  (bind _returnvalue_2 (Math|Float|MapRangeClamped _difficulty 0.1 1.0 5.0 5e+01))
  (bind _returnvalue_3 (|((round((value/5)))*5) _returnvalue_2))
  (switch int (Variables|/Game/Slappedy/GI_SlapInstance.GI_SlapInstance_C|GetPlayerAmount _asgi_slap_instance)
    (:1
      (CallFunction|SetMaxKills _returnvalue_3))
    (:2
      (CallFunction|SetMaxKills (|((round((value/5)))*5) (Math|Float|MapRangeClamped _difficulty 0.1 1.0 1e+01 5e+01))))
    (:3
      (CallFunction|SetMaxKills (|((round((value/5)))*5) (Math|Float|MapRangeClamped _difficulty 0.1 1.0 1e+01 5e+01))))
    (:4
      (CallFunction|SetMaxKills (|((round((value/5)))*5) (Math|Float|MapRangeClamped _difficulty 0.1 1.0 15.0 5e+01)))))
  (Development|PrintString (Utilities|String|ToString(Integer) _returnvalue_3)))