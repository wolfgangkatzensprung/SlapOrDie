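; BP_WallBouncer is a bounce pad that flings slappable actors along its arrow's horizontal direction when they overlap its box collider.
; The overlap plays a bounce montage and a pillow sound at world origin, then checks the actor's being-slapped state.
; Slapped actors get a multiplied horizontal force on their mesh's hips bone; otherwise, characters are launched with added fixed upward velocity.
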(event `self.BoxCollider.OnComponentBeginOverlap`
  (params (OverlappedComponent :type "PrimitiveComponent Object Reference") (OtherActor :type "Actor Object Reference") (OtherComp :type "PrimitiveComponent Object Reference") (OtherBodyIndex :type Integer) (bFromSweep :type Boolean) (SweepResult :type "HitResult Structure (by ref)"))
  (if (`KismetSystemLibrary.DoesImplementInterface` OtherActor "/Game/Slappedy/BPI_Slappable.BPI_Slappable_C")
    (`|ExecutionSequence`
      (:`then_0`
        (`|PlayMontage` (`self.SK_JumpPad`) "/Game/Level/Probs/Jump_Pad/Animation/Anim_WallBouncer_Montage.Anim_WallBouncer_Montage"))
      (:`then_1`
        (`GameplayStatics.PlaySoundAtLocation` "/Game/Audio/Sounds/Objects/MS_Pillow.MS_Pillow" (0.0 0.0 0.0) (struct) 1.0 1.0 0.0 null null null null)
        (bind _isbeingslapped (message `/Game/Slappedy/BPI_Slappable.GetIsBeingSlapped` OtherActor))
        (if _isbeingslapped
          (bind (_returnvalue_x _returnvalue_y) (`self.CalculateForceAndDirection`))
          (`PrimitiveComponent.AddForce` (`self.GetComponentByClass` OtherActor "/Script/Engine.MeshComponent") (* (`KismetMathLibrary.MakeVector` _returnvalue_x _returnvalue_y) (`self.ForceMultiplier`)) "hips" false)
          (else
            (bind _ascharacter (cast `Character` OtherActor))
            (bind (_returnvalue_x_2 _returnvalue_y_2) (`self.CalculateForceAndDirection`))
            (`Character.LaunchCharacter` _ascharacter (`KismetMathLibrary.MakeVector` _returnvalue_x_2 _returnvalue_y_2 450.0) false false)))))))

(fn `CalculateForceAndDirection`
  (returns (ReturnValue_X :type "Float (double-precision)") (ReturnValue_Y :type "Float (double-precision)"))
  (bind (_returnvalue_x _returnvalue_y) (`KismetMathLibrary.BreakVector` (* (`SceneComponent.GetForwardVector` (`self.Arrow`)) (`self.LaunchVelocity`))))
  (return _returnvalue_x _returnvalue_y))

(fn `UserConstructionScript`)