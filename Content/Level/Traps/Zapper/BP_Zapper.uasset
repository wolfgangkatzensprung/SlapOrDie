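; Zapper trap that charges when a BPI_Killable actor enters its trigger, then tries to kill the Characters inside.
; Overlap starts a charge with sound and two Niagara sparks, ignoring new entries until the delay ends.
; It then re-queries overlaps, sending TryKill to each Character and target lists to child BP_zapp actors for VFX, or plays a charge-lost sound if empty.
; Debug capsule and per-mesh electrified effects are unconnected.
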(event `self.Trigger.OnComponentEndOverlap`
  (params (OverlappedComponent :type "PrimitiveComponent Object Reference") (OtherActor :type "Actor Object Reference") (OtherComp :type "PrimitiveComponent Object Reference") (OtherBodyIndex :type Integer))
  ; Zapperarea wird verlassen
)

(event `self.ReceiveBeginPlay`
  ; Init
  (set `self.CanKill` false))

(event `self.Trigger.OnComponentBeginOverlap`
  (params (OverlappedComponent :type "PrimitiveComponent Object Reference") (OtherActor :type "Actor Object Reference") (OtherComp :type "PrimitiveComponent Object Reference") (OtherBodyIndex :type Integer) (bFromSweep :type Boolean) (SweepResult :type "HitResult Structure (by ref)"))
  ; Keep track of killable Actors in range
  (if (`KismetSystemLibrary.DoesImplementInterface` OtherActor "/Game/Slappedy/BPI_Killable.BPI_Killable_C")
    (`self.TryStartCharging`)))

(event `OnStartCharging`
  (bind _returnvalue (`SceneComponent.K2_GetComponentLocation` (`self.Trigger`)))
  ; Start charging
  (set `self.IsCharging` true)
  (`GameplayStatics.PlaySoundAtLocation` "/Game/Audio/Sounds/Objects/Zapper_Charge01.Zapper_Charge01" (0.0 0.0 0.0) (struct) 1.0 1.0 0.0 null null null null)
  (`|ExecutionSequence`
    (:`then_0`
      (`KismetSystemLibrary.Delay` (`self.ChargeTime`))
      (`self.OnFinishCharging`))
    (:`then_1`
      (`NiagaraFunctionLibrary.SpawnSystemAtLocation` "/Game/VFX/NS_charging_electric.NS_charging_electric" (+ _returnvalue (100.0 100.0 0.0)) (struct) (0.01 0.01 0.01)))
    (:`then_2`
      (`NiagaraFunctionLibrary.SpawnSystemAtLocation` "/Game/VFX/NS_charging_electric.NS_charging_electric" (+ _returnvalue (-100.0 -100.0 0.0)) (struct) (0.01 0.01 0.01)))))

(event `OnFinishCharging`
  ; Finish charging: Kill actors in range
  (set `self.IsCharging` false)
  (bind _entitiesinrange (`self.GetEntitiesInRange`))
  (if (`KismetArrayLibrary.Array_IsNotEmpty` _entitiesinrange)
    (`GameplayStatics.PlaySoundAtLocation` "/Game/Audio/Sounds/Objects/Zapp01.Zapp01" (0.0 0.0 0.0) (struct) 1.0 1.0 0.0 null null null null)
    (for _array_element _entitiesinrange
      (message `/Game/Slappedy/BPI_Killable.TryKill` _array_element self (`self.TrapId_0`) "NewEnumerator0")
      (for _array_element_2 (`self.GetAllChildActors` true)
        (bind _asbp_zapp (cast `/Game/VFX/BP_zapp` _array_element_2))
        (bind _entitiesinrange_2 (`self.GetEntitiesInRange`))
        (`/Game/VFX/BP_zapp.VFX_TraceTargets` _asbp_zapp _entitiesinrange_2)))
    (else
      (`GameplayStatics.PlaySoundAtLocation` "/Game/Audio/Sounds/Objects/Zapper_Charge_Lost01.Zapper_Charge_Lost01" (0.0 0.0 0.0) (struct) 1.0 1.0 0.0 null null null null))))

(fn `GetEntitiesInRange`
  (returns (EntitiesInRange :type "Array of Actor Object Reference"))
  (locals (Entities :type "Array of Actor Object Reference"))
  (bind _entities (`local.Entities`))
  (for _array_element (`self.GetOverlappingActors` "/Script/Engine.Character")
    (`KismetArrayLibrary.Array_Add` _entities _array_element))
  (return _entities))

(fn `TryStartCharging`
  (if (not (`self.IsCharging`))
    (`self.OnStartCharging`)))

(fn `UserConstructionScript`
  (`parent.UserConstructionScript`))