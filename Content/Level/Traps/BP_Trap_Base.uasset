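; BP_Trap_Base is a base trap actor that attempts to kill actors overlapping its Trigger component while CanKill is set.
; Overlapping actors that implement BPI_Killable receive a TryKill message with the trap as killer, plus a TrapId and DeathReason.
; When attached to a BP_TrapGroup_Base, the trap takes both values from that parent group, otherwise it uses its own.
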(event `self.Trigger.OnComponentBeginOverlap`
  (params (OverlappedComponent :type "PrimitiveComponent Object Reference") (OtherActor :type "Actor Object Reference") (OtherComp :type "PrimitiveComponent Object Reference") (OtherBodyIndex :type Integer) (bFromSweep :type Boolean) (SweepResult :type "HitResult Structure (by ref)"))
  (if (`self.CanKill`)
    (if (`KismetSystemLibrary.DoesImplementInterface` OtherActor "/Game/Slappedy/BPI_Killable.BPI_Killable_C")
      (bind (_trapid _deathreason) (`self.GetTrapIdAndDeathReason`))
      (message `/Game/Slappedy/BPI_Killable.TryKill` OtherActor self _trapid _deathreason))))

(fn `GetTrapIdAndDeathReason`
  (returns (TrapId :type String) (DeathReason :type "/Game/Slappedy/Enum_DeathReason Enum"))
  (bind _returnvalue (`self.GetAttachParentActor`))
  (`/Engine/EditorBlueprintResources/StandardMacros.IsValid` _returnvalue
    (:`Is Valid`
      (bind _asbp_trap_group_base (cast `/Game/Level/Traps/TrapGroups/BP_TrapGroup_Base` _returnvalue)
        (:`then`
          (return (`/Game/Level/Traps/TrapGroups/BP_TrapGroup_Base.TrapId` _asbp_trap_group_base) (`/Game/Level/Traps/TrapGroups/BP_TrapGroup_Base.DeathReason` _asbp_trap_group_base)))
        (:`CastFailed`
          _)))
    (:`Is Not Valid`
      _))
  (return (`self.TrapId`) (`self.DeathReason`)))

(fn `UserConstructionScript`)