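; BP_Cauldron is a level trap: an acid cauldron that delegates killing to a round death zone child actor.
; On BeginPlay it passes its death reason and trap ID to that BP_DeathZone_Round and binds to its OnKill event.
; Each kill plays the acid pool sound at the cauldron mesh placeholder's location, using a concurrency setting to manage overlapping sounds.
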(event `self.ReceiveBeginPlay`
  (bind _asbp_death_zone_round (cast `/Game/Level/BP_DeathZone_Round` (`ChildActorComponent.ChildActor` (`self.BP_DeathZone_Round`)) :!pure true))
  ; Acid Pool Sound
  (add `/Game/Level/BP_DeathZone_Round.OnKill` _asbp_death_zone_round (delegate `PlaySound`))
  (set `/Game/Level/BP_DeathZone_Round.DeathReason` (`self.DeathReason`) _asbp_death_zone_round)
  (set `/Game/Level/BP_DeathZone_Round.Trap Id` (`self.TrapId`) _asbp_death_zone_round))

(event `PlaySound`
  ; Acid Pool Sound
  (`GameplayStatics.PlaySoundAtLocation` "/Game/Audio/Sounds/Objects/AcidPool.AcidPool" (`SceneComponent.K2_GetComponentLocation` (`self.Cauldron_Placeholder`)) (struct) 1.0 1.0 0.0 null "/Game/Audio/SoundConcurrencys/AcidPitConcurrency.AcidPitConcurrency" null null))

(fn `UserConstructionScript`
  (`parent.UserConstructionScript`))