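; BP_GravityZone is a level trap that acts as a magnet, pushing physics-simulating killable actors in a set direction.
; Every tick it checks its overlapping actors for the BPI_Killable interface and for a mesh simulating physics at the "hips" bone.
; It applies GravityForce along the Arrow component's forward vector to that bone, as a mass-dependent force rather than an acceleration.
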(event `self.ReceiveTick`
  (params (DeltaSeconds :type "Float (single-precision)"))
  ; Magnet Force
  (for _array_element (`self.GetOverlappingActors` null)
    (if (`KismetSystemLibrary.DoesImplementInterface` _array_element "/Game/Slappedy/BPI_Killable.BPI_Killable_C")
      (bind _returnvalue (`self.GetComponentByClass` _array_element "/Script/Engine.MeshComponent"))
      (if (`SceneComponent.IsSimulatingPhysics` _returnvalue "hips")
        (`PrimitiveComponent.AddForce` _returnvalue (* (`SceneComponent.GetForwardVector` (`self.Arrow`)) (`self.GravityForce`)) "hips" false)))))

(fn `UserConstructionScript`)