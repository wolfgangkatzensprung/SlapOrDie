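; Base Blueprint for slappable breakable props that shatter into a Geometry Collection when slapped or overlapped by a slappable that is being slapped.
; Both triggers route through a server event to a multicast break, which swaps the static mesh for the collection and applies radial and directional impulses.
; Children override AAAOverrideGC to supply their fractured mesh.
; Breaking plays a sound, then destroys the actor after DecayTime.
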(event `Server_ApplySlap`
  (params (SlapForce :type "Vector Structure"))
  (`self.MC_Break` SlapForce))

(event `MC_Break`
  (params (Force :type "Vector Structure"))
  (if (not (`self.IsBroken`))
    (set `self.IsBroken` true)
    (`ActorComponent.K2_DestroyComponent` (`self.StaticMesh`))
    (bind _gc_component (`self.AAA_OverrideGC`))
    (`PrimitiveComponent.SetCollisionProfileName` _gc_component "NoCollision" false)
    (`PrimitiveComponent.AddRadialImpulse` _gc_component (`self.K2_GetActorLocation`) 200.0 2500000.0 "RIF_Constant" false)
    (`PrimitiveComponent.AddImpulse` _gc_component Force "None" false)
    (`self.OnBroken`)))

(event `OnBroken`
  (`/Engine/EditorBlueprintResources/StandardMacros.DoOnce` false
    (:`Completed`
      (`GameplayStatics.PlaySoundAtLocation` (`self.BreakSound`) (0.0 0.0 0.0) (struct) 1.0 1.0 0.0 null (`BlueprintMapLibrary.Map_Find` (`self.SoundToSoundCuncurrency`) (`self.BreakSound`)) null null)
      (`KismetSystemLibrary.Delay` (`self.DecayTime`))
      (`self.K2_DestroyActor`))))

(event `self.Col_Capsule.OnComponentBeginOverlap`
  (params (OverlappedComponent :type "PrimitiveComponent Object Reference") (OtherActor :type "Actor Object Reference") (OtherComp :type "PrimitiveComponent Object Reference") (OtherBodyIndex :type Integer) (bFromSweep :type Boolean) (SweepResult :type "HitResult Structure (by ref)"))
  (`self.OnCollisionOverlap` OtherActor))

(fn `AAA_OverrideGC`
  (returns (`GC Component` :type "GeometryCollectionComponent Object Reference"))
  (locals (Color :type "Color Structure"))
  ; Replace with the GC of the child mesh
  (bind _returnvalue (`AddComponent|NODE_AddGeometryCollectionComponent-1` :`RelativeTransform` (`SceneComponent.GetRelativeTransform` (`self.StaticMesh`))))
  (return _returnvalue))

(fn `GetCanBeSlapped`
  (returns (CanBeSlapped :type Boolean))
  (return (not (`self.IsBroken`))))

(fn `GetIsBeingSlapped`
  (returns (IsBeingSlapped :type Boolean))
  (return (`self.IsBroken`)))

(fn `OnCollisionOverlap`
  (params (`Other Actor` :type "Object Object Reference"))
  (if (`KismetSystemLibrary.DoesImplementInterface` `Other Actor` "/Game/Slappedy/BPI_Slappable.BPI_Slappable_C")
    (bind _isbeingslapped (message `/Game/Slappedy/BPI_Slappable.GetIsBeingSlapped` `Other Actor`))
    (if _isbeingslapped
      ; Break only radial from server
      (`self.Server_ApplySlap` (0.0 0.0 0.0)))))

(fn `TryApplySlap`
  (params (SlapForce :type "Vector Structure") (Slapper :type "Actor Object Reference"))
  (returns (SlapSucceeded :type Boolean))
  (if (`self.IsBroken`)
    (return false)
    (else
      (`self.Server_ApplySlap` SlapForce)
      (return true))))

(fn `UserConstructionScript`)