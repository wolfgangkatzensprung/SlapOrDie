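; Base Blueprint for breakable potions that adds a liquid splash when the potion breaks.
; On the MCBreak event it spawns a small Niagara splash above the root, tinted by a color variable and driven by the break force, then runs the parent break logic.
; It also overrides the geometry collection hook to add its own Geometry Collection component.
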(event `self.MC_Break`
  (params (Force :type "Vector Structure"))
  (`self.SpawnPotionParticles` Force)
  (`parent.MC_Break` Force))

(fn `AAA_OverrideGC`
  (returns (`GC Component` :type "GeometryCollectionComponent Object Reference"))
  (bind _returnvalue (`AddComponent|NODE_AddGeometryCollectionComponent-0`))
  (return _returnvalue))

(fn `SpawnPotionParticles`
  (params (ForceDirection :type "Vector Structure"))
  (bind _returnvalue (`NiagaraFunctionLibrary.SpawnSystemAtLocation` "/Game/VFX/NS_liquidsplashsmall.NS_liquidsplashsmall" (+ (`SceneComponent.K2_GetComponentLocation` (`self.DefaultSceneRoot`)) (0.0 0.0 80.0))))
  (`NiagaraComponent.SetVariableLinearColor` _returnvalue "Color" (`self.Color Linear`))
  (`NiagaraComponent.SetVariableVec3` _returnvalue "direction" ForceDirection))

(fn `UserConstructionScript`
  (`parent.UserConstructionScript`))