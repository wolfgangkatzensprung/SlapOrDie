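; Pole prop from a spline tool that strings four cable-component wires to the next pole in the chain.
; The construction script sets each cable's end to the matching connector on NextMesh, converted to actor-local space, and destroys all cables when that reference is invalid (last pole).
; Gravity is randomized or set per cable; shared width applies only in the random branch.
; ReattachCables branches to nothing, and the event graph is unused.
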(fn `UserConstructionScript`
  (bind _returnvalue (`KismetMathLibrary.RandomFloatInRange` 1.0 2.0))
  (bind _wirecable_3 (`self.WireCable_3`))
  (bind _wirecable_1 (`self.WireCable_1`))
  (bind _wirecable_2 (`self.WireCable_2`))
  (bind _wirecable_4 (`self.WireCable_4`))
  (bind _returnvalue_2 (`KismetMathLibrary.Conv_IntToDouble` (`self.Cable Width`)))
  (if (`self.ReattachCables`)
    _
    (else
      _))
  (`/Engine/EditorBlueprintResources/StandardMacros.IsValid` (`self.NextMesh`)
    (:`Is Valid`
      ;[1 1 1] Cable 1
      (set `CableComponent.EndLocation` (`KismetMathLibrary.InverseTransformLocation` (`self.GetTransform`) (`SceneComponent.K2_GetComponentLocation` (`/Game/Props/Splines/BP_SplineTool_Tiedtke_v001_UE4_27_2_Build/BP_SplineTool_Tiedtke_Wires_4_27_2.WireConnector_1` (`self.NextMesh`)))) (`self.WireCable_1`))
      ;[1 1 1] Cable 2
      (set `CableComponent.EndLocation` (`KismetMathLibrary.InverseTransformLocation` (`self.GetTransform`) (`SceneComponent.K2_GetComponentLocation` (`/Game/Props/Splines/BP_SplineTool_Tiedtke_v001_UE4_27_2_Build/BP_SplineTool_Tiedtke_Wires_4_27_2.WireConnector_2` (`self.NextMesh`)))) (`self.WireCable_2`))
      ;[1 1 1] Cable 3
      (set `CableComponent.EndLocation` (`KismetMathLibrary.InverseTransformLocation` (`self.GetTransform`) (`SceneComponent.K2_GetComponentLocation` (`/Game/Props/Splines/BP_SplineTool_Tiedtke_v001_UE4_27_2_Build/BP_SplineTool_Tiedtke_Wires_4_27_2.WireConnector_3` (`self.NextMesh`)))) (`self.WireCable_3`))
      ;[1 1 1] Cable 4
      (set `CableComponent.EndLocation` (`KismetMathLibrary.InverseTransformLocation` (`self.GetTransform`) (`SceneComponent.K2_GetComponentLocation` (`/Game/Props/Splines/BP_SplineTool_Tiedtke_v001_UE4_27_2_Build/BP_SplineTool_Tiedtke_Wires_4_27_2.WireConnector_4` (`self.NextMesh`)))) (`self.WireCable_4`))
      ;[1 1 1] Gravity & Cable Width
      (if (`self.RandomGravity`)
        (set `CableComponent.CableGravityScale` _returnvalue _wirecable_1)
        (set `CableComponent.CableWidth` _returnvalue_2 _wirecable_1)
        (set `CableComponent.CableGravityScale` _returnvalue _wirecable_2)
        (set `CableComponent.CableWidth` _returnvalue_2 _wirecable_2)
        (set `CableComponent.CableGravityScale` _returnvalue _wirecable_3)
        (set `CableComponent.CableWidth` _returnvalue_2 _wirecable_3)
        (set `CableComponent.CableGravityScale` _returnvalue _wirecable_4)
        (set `CableComponent.CableWidth` _returnvalue_2 _wirecable_4)
        (else
          (set `CableComponent.CableGravityScale` (`self.Cable_1_Gravity`) (`self.WireCable_1`))
          (set `CableComponent.CableGravityScale` (`self.Cable_2_Gravity`) (`self.WireCable_2`))
          (set `CableComponent.CableGravityScale` (`self.Cable_3_Gravity`) (`self.WireCable_3`))
          (set `CableComponent.CableGravityScale` (`self.Cable_4_Gravity`) (`self.WireCable_4`)))))
    (:`Is Not Valid`
      ;[1 1 1] Last Pole Destroy Cables
      (`ActorComponent.K2_DestroyComponent` (`self.WireCable_4`))
      (`ActorComponent.K2_DestroyComponent` (`self.WireCable_3`))
      (`ActorComponent.K2_DestroyComponent` (`self.WireCable_1`))
      (`ActorComponent.K2_DestroyComponent` (`self.WireCable_2`)))))